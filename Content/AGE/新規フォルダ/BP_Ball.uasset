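; BP_Ball is a ball actor that jumps upward when BP_SARA touches it.
; An overlap on the Sphere1 component checks that the other actor is BP_SARA, then raises the Sphere component by a random height along world Z.
; The move is an instant, swept location change rather than a physics impulse, so blocking geometry can stop it.
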(event OnComponentBeginOverlap(Sphere1)
  (params (OverlappedComponent :type Primitive%20Component%20Object%20Reference) (OtherActor :type Actor%20Object%20Reference) (OtherComp :type Primitive%20Component%20Object%20Reference) (OtherBodyIndex :type Integer) (bFromSweep :type Boolean) (SweepResult :type Hit%20Result%20Structure%20%28by%20ref%29))
  (bind _sphere (Variables|Default|GetSphere))
  (bind _returnvalue (Transformation|GetWorldLocation _sphere))
  (bind (_x _y _z) (Math|Vector|BreakVector _returnvalue))
  (if (== OtherActor "/Game/AGE/新規フォルダ/BP_SARA.BP_SARA")
    (Transformation|SetWorldLocation _sphere (Math|Vector|MakeVector _x _y (+ _z (Math|Conversions|ToFloat(Integer) (+ (Math|Random|RandomInteger 300) 100)))) true false)))

(event EventBeginPlay)

(event Collision|EventActorBeginOverlap
  (params (OtherActor :type Actor%20Object%20Reference)))

(event EventTick
  (params (DeltaSeconds :type Float%20%28single-precision%29)))

(fn ConstructionScript)